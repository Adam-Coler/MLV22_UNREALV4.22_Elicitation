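; Magic Leap hand-gesture reader that registers itself with the game instance and manages which static gestures are tracked and their confidence threshold.
; Gesture key presses fire OnGestureDetected, always with hand 0, whose bound handler refreshes both hands' stored gestures and broadcasts GestureUpdated.
; Helper functions query gestures, toggle tracking and return hand position from the first available keypoint.
; Hand visibility outputs are always false, and IsGestureActive always reports LeftHand.
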(event Custom|SetCurrentGestures
  (params (Gesture :type EHandTrackingGesture%20Enum :default "Finger") (Hand :type Byte))
  ;[1 0.1853 0] Save current gestures for each hand
  (Gestures|UpdateCurrentGestures))

(event EventBeginPlay
  ;[0.165 1 0.1379] Initialize
  (Utilities|FlowControl|Sequence
    (:then_0
      (Input|EnableInput (Game|GetPlayerController 0)))
    (:then_1
      (Class|MagicLeapHandTrackingFunctionLibrary|SetConfiguration (Variables|Gestures|GetActiveStaticGestures) "NoFilter" "NoFilter" true)
      (for _array_element (Variables|Gestures|GetActiveStaticGestures)
        (Class|MagicLeapHandTrackingFunctionLibrary|SetStaticGestureConfidenceThreshold _array_element (Variables|Gestures|GetGestureConfidenceThreshold))))
    (:then_2
      (EventDispatchers|BindEventtoOnGestureDetected (delegate Custom|SetCurrentGestures)))
    (:then_3
      (bind _gameinstanacear (CallFunction|FGetGameInstance))
      (Variables|/Game/GameModes/Game_Instance_AR_Affordances.Game_Instance_AR_Affordances_C|SetGestureReader _gameinstanacear self))))

(event EventEndPlay
  (params (EndPlayReason :type EEndPlayReason%20Enum :default "Destroyed"))
  ;[1 0.165 0.1379] Finalize
  (Class|MagicLeapHandTrackingFunctionLibrary|SetConfiguration (Utilities|Array|MakeArray "NoHand") "NoFilter" "NoFilter" true))

(event Input|KeyboardEvents|MagicLeapLeftThumb
  (params (Key :type Key%20Structure))
  ;[0.1451 0.003922 0.003922] Left Hand - Gesture Events
  (:Pressed
    (Default|CallOnGestureDetected "Thumb")))

(event Input|KeyboardEvents|MagicLeapLeftC
  (params (Key :type Key%20Structure))
  ;[0.1451 0.003922 0.003922] Left Hand - Gesture Events
  (:Pressed
    (Default|CallOnGestureDetected "C")))

(event Input|KeyboardEvents|MagicLeapRightFinger
  (params (Key :type Key%20Structure))
  ;[0.1441 0.003677 0.003677] Right Hand - Gesture Events
  (:Pressed
    (Default|CallOnGestureDetected "Finger")))

(event Input|KeyboardEvents|MagicLeapRightFist
  (params (Key :type Key%20Structure))
  ;[0.1441 0.003677 0.003677] Right Hand - Gesture Events
  (:Pressed
    (Default|CallOnGestureDetected "Fist")))

(event Input|KeyboardEvents|MagicLeapRightPinch
  (params (Key :type Key%20Structure))
  ;[0.1441 0.003677 0.003677] Right Hand - Gesture Events
  (:Pressed
    (Default|CallOnGestureDetected "Pinch")))

(event Input|KeyboardEvents|MagicLeapRightThumb
  (params (Key :type Key%20Structure))
  ;[0.1441 0.003677 0.003677] Right Hand - Gesture Events
  (:Pressed
    (Default|CallOnGestureDetected "Thumb")))

(event Input|KeyboardEvents|MagicLeapLeftFinger
  (params (Key :type Key%20Structure))
  ;[0.1451 0.003922 0.003922] Left Hand - Gesture Events
  (:Pressed
    (Default|CallOnGestureDetected "Finger")))

(event Input|KeyboardEvents|MagicLeapRightL
  (params (Key :type Key%20Structure))
  ;[0.1441 0.003677 0.003677] Right Hand - Gesture Events
  (:Pressed
    (Default|CallOnGestureDetected "L")))

(event Input|KeyboardEvents|MagicLeapRightOpenHandBack
  (params (Key :type Key%20Structure))
  ;[0.1441 0.003677 0.003677] Right Hand - Gesture Events
  (:Pressed
    (Default|CallOnGestureDetected "OpenHandBack")))

(event Input|KeyboardEvents|MagicLeapRightOk
  (params (Key :type Key%20Structure))
  ;[0.1441 0.003677 0.003677] Right Hand - Gesture Events
  (:Pressed
    (Default|CallOnGestureDetected "Ok")))

(event Input|KeyboardEvents|MagicLeapRightC
  (params (Key :type Key%20Structure))
  ;[0.1441 0.003677 0.003677] Right Hand - Gesture Events
  (:Pressed
    (Default|CallOnGestureDetected "C")))

(event Input|KeyboardEvents|MagicLeapRightNoHand
  (params (Key :type Key%20Structure))
  ;[0.1441 0.003677 0.003677] Right Hand - Gesture Events
  (:Pressed
    (Default|CallOnGestureDetected "NoHand")))

(event Input|KeyboardEvents|MagicLeapLeftFist
  (params (Key :type Key%20Structure))
  ;[0.1451 0.003922 0.003922] Left Hand - Gesture Events
  (:Pressed
    (Default|CallOnGestureDetected "Fist")))

(event Input|KeyboardEvents|MagicLeapLeftL
  (params (Key :type Key%20Structure))
  ;[0.1451 0.003922 0.003922] Left Hand - Gesture Events
  (:Pressed
    (Default|CallOnGestureDetected "L")))

(event Input|KeyboardEvents|MagicLeapLeftNoHand
  (params (Key :type Key%20Structure))
  ;[0.1451 0.003922 0.003922] Left Hand - Gesture Events
  (:Pressed
    (Default|CallOnGestureDetected "NoHand")))

(event Input|KeyboardEvents|MagicLeapLeftOk
  (params (Key :type Key%20Structure))
  ;[0.1451 0.003922 0.003922] Left Hand - Gesture Events
  (:Pressed
    (Default|CallOnGestureDetected "Ok")))

(event Input|KeyboardEvents|MagicLeapLeftOpenHandBack
  (params (Key :type Key%20Structure))
  ;[0.1451 0.003922 0.003922] Left Hand - Gesture Events
  (:Pressed
    (Default|CallOnGestureDetected "OpenHandBack")))

(event Input|KeyboardEvents|MagicLeapLeftPinch
  (params (Key :type Key%20Structure))
  ;[0.1451 0.003922 0.003922] Left Hand - Gesture Events
  (:Pressed
    (Default|CallOnGestureDetected "Pinch")))

(fn ConstructionScript)

(fn IsGestureActive
  (params (Gesture :type EHandTrackingGesture%20Enum :default "Finger") (Hand :type E_HandType%20Enum :default "NewEnumerator0"))
  (bind _currentleftgesture (Variables|Gestures|GetCurrentLeftGesture))
  (bind _currentrightgesture (Variables|Gestures|GetCurrentRightGesture))
  (bind _returnvalue (Utilities|Enum|Equal(Enum) Gesture _currentrightgesture))
  (bind _returnvalue_2 (Utilities|Enum|Equal(Enum) _currentleftgesture Gesture))
  (switch Utilities|FlowControl|Switch|SwitchonE_HandType Hand
    (:NewEnumerator0
      ;[1 1 1] Matching hand and gesture
      (return (Utilities|Enum|Equal(Enum) (Variables|Gestures|GetCurrentLeftGesture) Gesture) "NewEnumerator0"))
    (:NewEnumerator1
      (return (Utilities|Enum|Equal(Enum) Gesture (Variables|Gestures|GetCurrentRightGesture)) "NewEnumerator0"))
    (:NewEnumerator2
      ;[1 1 1] Check if any hand matches gesture and report that info back to caller
      (if (and _returnvalue_2 _returnvalue)
        (return true "NewEnumerator0")
        (elif _returnvalue_2
          (return true "NewEnumerator0")
          (else
            (return _returnvalue "NewEnumerator0")))))))

(fn GetCurrentGesture
  (params (Hand :type E_HandType%20Enum :default "NewEnumerator0"))
  (bind _currentleftgesture (Variables|Gestures|GetCurrentLeftGesture))
  (switch Utilities|FlowControl|Switch|SwitchonE_HandType Hand
    (:NewEnumerator0
      (return (Variables|Gestures|GetCurrentLeftGesture)))
    (:NewEnumerator1
      (return (Variables|Gestures|GetCurrentRightGesture)))
    (:NewEnumerator2
      ;[1 1 1] When requesting both hands, try to give left gesture if valid, otherwise give whatever right is
      (return (select (Utilities|Enum|Equal(Enum) _currentleftgesture "NoHand") (Variables|Gestures|GetCurrentRightGesture) _currentleftgesture)))))

(fn UpdateCurrentGestures
  (Utilities|FlowControl|Sequence
    (:then_0
      (bind _gesture (Class|MagicLeapHandTrackingFunctionLibrary|GetCurrentGesture "Left"))
      (bind _output_get (Variables|Gestures|SetCurrentLeftGesture _gesture)))
    (:then_1
      (bind _gesture_2 (Class|MagicLeapHandTrackingFunctionLibrary|GetCurrentGesture "Right"))
      (bind _output_get_2 (Variables|Gestures|SetCurrentRightGesture _gesture_2)))
    (:then_2
      (Default|CallGestureUpdated))))

(fn SetGestureTrackingStatus
  (params (Gesture :type EHandTrackingGesture%20Enum :default "Finger") (Tracked :type Boolean))
  (bind _activestaticgestures (Variables|Gestures|GetActiveStaticGestures))
  (bind _activestaticgestures_2 (Variables|Gestures|GetActiveStaticGestures))
  (bind _returnvalue (Utilities|Array|ContainsItem _activestaticgestures Gesture))
  (if Tracked
    ;[1 1 1] Only take action when state has changed
    (if (not _returnvalue)
      ;[1 1 1] Update active gestures
      (Utilities|FlowControl|Sequence
        (:then_0
          (Utilities|Array|Add _activestaticgestures_2 Gesture))
        (:then_1
          (Class|MagicLeapHandTrackingFunctionLibrary|SetConfiguration (Variables|Gestures|GetActiveStaticGestures) "NoFilter" "NoFilter" true :!label _label))))
    (elif _returnvalue
      (Utilities|FlowControl|Sequence
        (:then_0
          (Utilities|Array|RemoveItem _activestaticgestures_2 Gesture))
        (:then_1
          (goto _label))))))

(fn GetActiveGestures
  (return (Variables|Gestures|GetActiveStaticGestures)))

(fn SetGestureConfidenceThreshold
  (params (NewConfidence :type Float%20%28single-precision%29))
  (Utilities|FlowControl|Sequence
    (:then_0
      (bind _output_get (Variables|Gestures|SetGestureConfidenceThreshold NewConfidence)))
    (:then_1
      (for _array_element (Variables|Gestures|GetActiveStaticGestures)
        (Class|MagicLeapHandTrackingFunctionLibrary|SetStaticGestureConfidenceThreshold _array_element _output_get)))))

(fn GetHandPosition
  (params (Hand :type E_HandType%20Enum :default "NewEnumerator0"))
  (bind _array (Utilities|Array|MakeArray "Thumb_Tip" "Index_Tip" "Middle_Tip" "Ring_Tip" "Pinky_Tip" "Hand_Center"))
  (switch Utilities|FlowControl|Switch|SwitchonE_HandType Hand
    (:NewEnumerator0
      (bind _array_element (Utilities|Array|ForEachLoopwithBreak _array :!label _label)
        (:LoopBody
          (bind (_transform _returnvalue) (Class|MagicLeapHandTrackingFunctionLibrary|GetGestureKeypointTransform "Left" _array_element "Tracking"))
          (if _returnvalue
            (goto _label Break)))
        (:Completed
          (return (.location _transform) false "0, 0, 0" false))))
    (:NewEnumerator1
      (bind _array_element_2 (Utilities|Array|ForEachLoopwithBreak _array :!label _label_2)
        (:LoopBody
          (bind (_transform_2 _returnvalue_2) (Class|MagicLeapHandTrackingFunctionLibrary|GetGestureKeypointTransform "Right" _array_element_2 "Tracking"))
          (if _returnvalue_2
            (goto _label_2 Break)))
        (:Completed
          (return "0, 0, 0" false (.location _transform_2) false))))))