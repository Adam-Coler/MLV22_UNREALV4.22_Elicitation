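; XR pawn for positioning a shelf with a right-hand motion controller (Magic Leap bindings) before loading MapPractice.
; Controller buttons and thumbstick nudge or yaw the GameInstance's shelf, while a trigger click snaps it to a line-trace hit.
; A trigger double-click, or deflected thumbstick press, toggles mesh scanning, destroys the pawn, saves the shelf transform and changes level.
; A delay-based macro separates single from double clicks, and Tick stretches a beam mesh to the traced surface.
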(event Custom|HapticMed
  (Class|MagicLeapControllerFunctionLibrary|PlayHapticPattern "Right" "Buzz" "Medium"))

(event EventBeginPlay
  (bind _motioncontroller (Variables|Default|GetMotionController))
  ;[0.06772 1 0.2163] Begin Play
  (Utilities|FlowControl|Sequence
    (:then_0
      (Utilities|IsValid _motioncontroller
        (:Is%20Valid
          (Variables|/Script/HeadMountedDisplay.MotionControllerComponent|SetMotionSource _motioncontroller "Right")
          (CallFunction|FPrint "MapLoadActor->controller set"))))
    (:then_1
      (bind _gameinstanacear (CallFunction|FGetGameInstance))
      (Variables|Default|SetGameInstance _gameinstanacear)
      (CallFunction|FPrint "MapLoadActor->GameInstance set"))
    (:then_2
      (Utilities|FlowControl|Delay 0.2)
      (Variables|Default|SetShelf (Variables|/Game/GameModes/Game_Instance_AR_Affordances.Game_Instance_AR_Affordances_C|GetShelf (Variables|Default|GetGameInstance)))
      (CallFunction|FPrint "MapLoadActor->Shelf Set"))))

(event Collision|EventActorBeginOverlap
  (params (OtherActor :type Actor%20Object%20Reference)))

(event EventTick
  (params (DeltaSeconds :type Float%20%28single-precision%29))
  (CallFunction|FDrawRayTraceControllertoCollision))

(event Input|KeyboardEvents|MotionControllerRightThumbstick
  (params (Key :type Key%20Structure))
  ;[1 0.0389 0.1086] Remote Bindings
  ;;[1 1 1] place / confirm
  (:Pressed
    (Math|Float|CompareFloat (Math|Float|Absolute(Float) (Class|Actor|GetInputAxisKeyValue)) 0.5
      (:>
        (Default|ToggleScan (Variables|/Game/GameModes/Game_Instance_AR_Affordances.Game_Instance_AR_Affordances_C|GetMeshing (Variables|Default|GetGameInstance)))
        (Actor|DestroyActor)
        (CallFunction|FNextLevel)))))

(event Input|KeyboardEvents|MotionControllerRightThumbstick
  (params (Key :type Key%20Structure))
  (bind _returnvalue (Class|Actor|GetInputAxisKeyValue))
  (bind _returnvalue_2 (Class|Actor|GetInputAxisKeyValue))
  (bind _shelf (Variables|Default|GetShelf))
  (bind _returnvalue_3 (Transformation|GetActorLocation _shelf))
  (bind _returnvalue_4 (Transformation|GetActorLocation _shelf))
  ;[1 0.0389 0.1086] Remote Bindings
  ;;[1 1 1] translate x y z
  (:Pressed
    (Utilities|FlowControl|Sequence
      (:then_0
        (Math|Float|CompareFloat (Math|Float|Absolute(Float) _returnvalue) 0.5
          (:>
            (Transformation|SetActorRelativeLocation _shelf (Math|Vector|MakeVector (.x _returnvalue_4) (+ (.y _returnvalue_4) (* _returnvalue 1.0)) (.z _returnvalue_4))))))
      (:then_1
        (Math|Float|CompareFloat (Math|Float|Absolute(Float) _returnvalue_2) 0.5
          (:>
            (Transformation|SetActorRelativeLocation _shelf (Math|Vector|MakeVector (+ (.x _returnvalue_3) (* _returnvalue_2 1.0)) (.y _returnvalue_3) (.z _returnvalue_3)))))))))

(event Input|KeyboardEvents|MotionControllerRightTrigger
  (params (Key :type Key%20Structure))
  ;[1 0.0389 0.1086] Remote Bindings
  ;;[1 1 1] place / confirm
  (:Pressed
    (CallFunction|HapticMed)
    (Utilities|DetectDoubleClick
      (:Double%20Click
        (Default|ToggleScan (Variables|/Game/GameModes/Game_Instance_AR_Affordances.Game_Instance_AR_Affordances_C|GetMeshing (Variables|Default|GetGameInstance)))
        (Actor|DestroyActor)
        (CallFunction|FNextLevel))
      (:Single%20Click
        (bind (_hitcomponent _objecthit _location) (CallFunction|FLineTracefromController))
        (if _objecthit
          (Transformation|SetActorLocation (Variables|Default|GetShelf) _location false false))))))

(event Input|KeyboardEvents|MotionControllerRightShoulder
  (params (Key :type Key%20Structure))
  (bind _shelf (Variables|Default|GetShelf))
  (bind _returnvalue (Transformation|GetActorRotation _shelf))
  ;[1 0.0389 0.1086] Remote Bindings
  ;;[1 1 1] rotate
  (:Pressed
    (CallFunction|HapticMed)
    (Utilities|DetectDoubleClick
      (:Double%20Click
        (Transformation|SetActorRelativeRotation _shelf (Math|Rotator|MakeRotator (.roll _returnvalue) (.pitch _returnvalue) (+ (.yaw _returnvalue) -2.0))))
      (:Single%20Click
        (Transformation|SetActorRelativeRotation _shelf (Math|Rotator|MakeRotator (.roll _returnvalue) (.pitch _returnvalue) (+ (.yaw _returnvalue) 2.0)))))))

(event Input|KeyboardEvents|MagicLeapRightHomeButton
  (params (Key :type Key%20Structure))
  (bind _shelf (Variables|Default|GetShelf))
  (bind _returnvalue (Transformation|GetActorLocation _shelf))
  ;[1 0.0389 0.1086] Remote Bindings
  ;;[1 1 1] translate  z single double
  (:Pressed
    (CallFunction|HapticMed)
    (Utilities|DetectDoubleClick
      (:Double%20Click
        (Transformation|SetActorRelativeLocation _shelf (Math|Vector|MakeVector (.x _returnvalue) (.y _returnvalue) (+ (.z _returnvalue) 1.0))))
      (:Single%20Click
        (Transformation|SetActorRelativeLocation _shelf (Math|Vector|MakeVector (.x _returnvalue) (.y _returnvalue) (+ (.z _returnvalue) -1.0)))))))

(fn ConstructionScript)

(fn FLineTracefromController
  (bind _motioncontroller (Variables|Default|GetMotionController))
  (bind _returnvalue (Transformation|GetWorldLocation _motioncontroller))
  (bind (_outhit _returnvalue_2) (Collision|LineTraceByChannel _returnvalue (+ _returnvalue (* (Math|Vector|GetForwardVector _motioncontroller) (Variables|Trace|GetTraceDistance))) "TraceTypeQuery1" false 0 "ForDuration" true "(R=0.000000,G=0.500000,B=1.000000,A=1.000000)"))
  (return (.hitcomponent _outhit) _returnvalue_2 (.location _outhit)))

(fn FDrawRayTraceControllertoCollision
  (bind _motioncontroller (Variables|Default|GetMotionController))
  (bind _tracemeshbeam (Variables|Default|GetTraceMeshBeam))
  (bind _beamlength (Variables|Trace|GetBeamLength))
  (bind _beamthickness (Variables|Trace|GetBeamThickness))
  (bind _returnvalue (Transformation|GetWorldLocation _motioncontroller))
  (bind _returnvalue_2 (* _beamthickness 0.01))
  (if (Variables|Trace|GetIsBeamOn)
    (bind _outhit (Collision|LineTraceByChannel _returnvalue (+ _returnvalue (* (Math|Vector|GetForwardVector _motioncontroller) (Variables|Trace|GetTraceDistance))) "TraceTypeQuery1" false 0 "None" true "(R=0.000000,G=0.500000,B=1.000000,A=1.000000)"))
    (if (.bblockinghit _outhit)
      (bind _output_get (Variables|Trace|SetBeamLengthNew (* (* (/ (- (.distance _outhit) (Variables|Trace|GetBeamOrginOffset)) _beamlength) _beamlength) 0.01)))
      (Transformation|SetWorldScale3D _tracemeshbeam (Math|Vector|MakeVector _returnvalue_2 _returnvalue_2 _output_get))
      (else
        (bind _output_get_2 (Variables|Trace|SetBeamLengthNew (* (Variables|Trace|GetBeamLength) 0.01)))
        (Transformation|SetWorldScale3D _tracemeshbeam (Math|Vector|MakeVector _returnvalue_2 _returnvalue_2 _output_get_2))))
    (Transformation|SetRelativeLocation _tracemeshbeam (Math|Vector|MakeVector (Math|Float|Absolute(Float) (+ (* (Variables|Trace|GetBeamLengthNew) 0.5 1e+02) (Variables|Trace|GetBeamOrginOffset))) 0.0 0.0) false false)))

(fn FNextLevel
  (Variables|/Game/GameModes/Game_Instance_AR_Affordances.Game_Instance_AR_Affordances_C|SetShelf_Transform (Variables|Default|GetGameInstance) (Transformation|GetActorTransform (Variables|Default|GetShelf)))
  (Game|OpenLevel(byName) "MapPractice"))