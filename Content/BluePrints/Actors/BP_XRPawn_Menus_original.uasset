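; XR menu pawn that shows the title screen on a widget and hands over to the participant pawn on a thumbs-up.
; Each tick the widget soft-locks in front of the camera, lerping toward it and facing it.
; Gesture reader updates check both hands for the Thumb pose, then ask the game instance to switch pawns.
; The soft-lock function and double-click macro are not called in the event graph.
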(event Custom|GestureUpdated
  ;[0.06772 1 0.2163] Begin Play
  (CallFunction|CheckforThumbsUp))

(event Custom|WidgetSoftlock
  (params (DeltaSeconds :type Float%20%28single-precision%29))
  (bind _returnvalue (Game|GetPlayerCameraManager 0))
  (bind _widget (Variables|Default|GetWidget))
  (bind _returnvalue_2 (Camera|GetCameraLocation _returnvalue))
  ;[1 1 1] WidgetSoftLock
  (bind _output_get (Variables|WidgetSoftLock|SetLocationTarget (+ _returnvalue_2 (* (Transformation|GetActorForwardVector _returnvalue) (Variables|WidgetSoftLock|GetWidgetDistance)))))
  (bind _output_get_2 (Variables|WidgetSoftLock|SetLocationCurrent (Math|Vector|Lerp(Vector) (Variables|WidgetSoftLock|GetLocationCurrent) _output_get (* DeltaSeconds (Variables|WidgetSoftLock|GetWidgetInterpSpeed)))))
  (Transformation|SetWorldLocation _widget _output_get_2 false false)
  (Transformation|SetWorldRotation _widget (Math|Rotator|FindLookatRotation (Transformation|GetWorldLocation _widget) _returnvalue_2) false false))

(event Custom|CheckForThumbsUp
  (bind _gesturereader (Variables|Default|GetGestureReader))
  ;[0.2413 0.438 1] Thumbs Up Load Next Pawn
  (switch Utilities|FlowControl|Switch|SwitchonEHandTrackingGesture (Default|GetCurrentGesture _gesturereader "NewEnumerator1")
    (:Finger
      (switch Utilities|FlowControl|Switch|SwitchonEHandTrackingGesture (Default|GetCurrentGesture _gesturereader "NewEnumerator0") :!label _label
        (:Thumb
          _)))
    (:Fist
      (goto _label))
    (:Pinch
      (goto _label))
    (:Thumb
      _)
    (:L
      (goto _label))
    (:OpenHandBack
      (goto _label))
    (:Ok
      (goto _label))
    (:C
      (goto _label))
    (:NoPose
      (goto _label))
    (:NoHand
      (goto _label)))
  (CallFunction|FLoadNextPawn))

(event EventBeginPlay
  ;[0.06772 1 0.2163] Begin Play
  (Utilities|FlowControl|Sequence
    (:then_0
      (bind _returnvalue (UserInterface|CreateWidget "/Game/Menus/W_01_Page_TitleScreen.W_01_Page_TitleScreen_C"))
      (Variables|Default|SetWidget_TitleScreen _returnvalue))
    (:then_1
      (UserInterface|SetWidget (Variables|Default|GetWidget) (Variables|Default|GetWidget_TitleScreen)))
    (:then_2
      (Transformation|SetWorldScale3D (Variables|Default|GetWidget) (Math|Conversions|ToVector(Float) (Variables|WidgetSoftLock|GetWidgetScale))))
    (:then_3
      (bind _gesturereader (CallFunction|FGetGestureReader))
      (bind _output_get (Variables|Default|SetGestureReader _gesturereader))
      (EventDispatchers|BindEventtoGestureUpdated _output_get (delegate Custom|GestureUpdated)))))

(event EventTick
  (params (DeltaSeconds :type Float%20%28single-precision%29))
  ;[1 0.02717 0.2379] Event Tick
  (CallFunction|WidgetSoftlock DeltaSeconds))

(fn ConstructionScript)

(fn FSoftLock
  (params (Component :type Scene%20Component%20Object%20Reference))
  (bind _returnvalue (Game|GetPlayerCameraManager 0))
  (bind _returnvalue_2 (Camera|GetCameraLocation _returnvalue))
  (bind _output_get (Variables|WidgetSoftLock|SetLocationTarget (+ _returnvalue_2 (* (Transformation|GetActorForwardVector _returnvalue) (Variables|WidgetSoftLock|GetWidgetDistance)))))
  (bind _output_get_2 (Variables|WidgetSoftLock|SetLocationCurrent (Math|Vector|Lerp(Vector) (Variables|WidgetSoftLock|GetLocationCurrent) _output_get (* (Utilities|Time|GetWorldDeltaSeconds) (Variables|WidgetSoftLock|GetWidgetInterpSpeed)))))
  (Transformation|SetWorldLocation Component _output_get_2 false false)
  (Transformation|SetWorldRotation Component (Math|Rotator|FindLookatRotation (Transformation|GetWorldLocation Component) _returnvalue_2) false false))

(fn FLoadNextPawn
  (bind _gameinstanacear (CallFunction|FGetGameInstance))
  (Variables|/Game/GameModes/Game_Instance_AR_Affordances.Game_Instance_AR_Affordances_C|SetCurrentPawn _gameinstanacear self)
  (Default|FMenuPawntoParticipantPawn _gameinstanacear))