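; XR pawn for the instructions scene that shows paged text on a world-space W_InstructionsScreen widget, then opens MapMain after the last page.
; Right trigger or Space steps CurrentPage through the E_Instructions_paths enum and loads that page's text from file into the widget via an event dispatcher.
; On Tick, the widget soft-locks ahead of the camera, lerping toward a point at WidgetDistance and rotating to face the viewer.
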(event Custom|ProgressScreens
  ;[1 1 1] Progress Screens
  (bind (_path _islast) (CallFunction|FGetNextInstructionsPage (Variables|Default|GetCurrentPage)))
  (Variables|Default|SetCurrentPage _path)
  (if _islast
    (Game|OpenLevel(byName) "MapMain")
    (else
      (CallFunction|FUpdateTextonWidgetViaEventDispatch (Utilities|Text|ToText(String) (.SaveTextA (Class|CBlueprintFunctionLibrary|FileLoadString (Utilities|String|EnumtoString (Variables|Default|GetCurrentPage)))))))))

(event Custom|WidgetSoftlock
  (params (DeltaSeconds :type Float%20%28single-precision%29))
  (bind _returnvalue (Game|GetPlayerCameraManager 0))
  (bind _widget (Variables|Default|GetWidget))
  (bind _returnvalue_2 (Camera|GetCameraLocation _returnvalue))
  ;[1 1 1] WidgetSoftLock
  (bind _output_get (Variables|WidgetSoftLock|SetLocationTarget (+ _returnvalue_2 (* (Transformation|GetActorForwardVector _returnvalue) (Variables|WidgetSoftLock|GetWidgetDistance)))))
  (bind _output_get_2 (Variables|WidgetSoftLock|SetLocationCurrent (Math|Vector|Lerp(Vector) (Variables|WidgetSoftLock|GetLocationCurrent) _output_get (* DeltaSeconds (Variables|WidgetSoftLock|GetWidgetInterpSpeed)))))
  (Transformation|SetWorldLocation _widget _output_get_2 false false)
  (Transformation|SetWorldRotation _widget (Math|Rotator|FindLookatRotation (Transformation|GetWorldLocation _widget) _returnvalue_2) false false))

(event EventBeginPlay
  (bind _widget (Variables|Default|GetWidget))
  ;[0.06772 1 0.2163] Begin Play
  (bind _returnvalue (UserInterface|CreateWidget "/Game/Menus/W_InstructionsScreen.W_InstructionsScreen_C"))
  (UserInterface|SetWidget _widget _returnvalue)
  (Transformation|SetWorldScale3D _widget (Math|Conversions|ToVector(Float) 0.05))
  (CallFunction|FUpdateTextonWidgetViaEventDispatch (Utilities|Text|ToText(String) (.SaveTextA (Class|CBlueprintFunctionLibrary|FileLoadString (Utilities|String|EnumtoString (Variables|Default|GetCurrentPage))))))
  (Pawn|Possess (Game|GetPlayerController 0) self)
  (Variables|/Script/HeadMountedDisplay.MotionControllerComponent|SetMotionSource (Variables|Default|GetMotionController) "Right")
  (CallFunction|FPrint "BP_Instructions->controller set"))

(event EventTick
  (params (DeltaSeconds :type Float%20%28single-precision%29))
  ;[1 0.02717 0.2379] Event Tick
  (CallFunction|WidgetSoftlock DeltaSeconds))

(event Input|KeyboardEvents|SpaceBar
  (params (Key :type Key%20Structure))
  ;[1 1 1] Inputs
  (:Pressed
    (CallFunction|ProgressScreens)))

(event Input|KeyboardEvents|MotionControllerRightTrigger
  (params (Key :type Key%20Structure))
  ;[1 1 1] Inputs
  (:Pressed
    (CallFunction|ProgressScreens)))

(fn ConstructionScript)

(fn FSoftLock
  (params (Component :type Scene%20Component%20Object%20Reference))
  (bind _returnvalue (Game|GetPlayerCameraManager 0))
  (bind _returnvalue_2 (Camera|GetCameraLocation _returnvalue))
  (bind _output_get (Variables|WidgetSoftLock|SetLocationTarget (+ _returnvalue_2 (* (Transformation|GetActorForwardVector _returnvalue) (Variables|WidgetSoftLock|GetWidgetDistance)))))
  (bind _output_get_2 (Variables|WidgetSoftLock|SetLocationCurrent (Math|Vector|Lerp(Vector) (Variables|WidgetSoftLock|GetLocationCurrent) _output_get (* (Utilities|Time|GetWorldDeltaSeconds) (Variables|WidgetSoftLock|GetWidgetInterpSpeed)))))
  (Transformation|SetWorldLocation Component _output_get_2 false false)
  (Transformation|SetWorldRotation Component (Math|Rotator|FindLookatRotation (Transformation|GetWorldLocation Component) _returnvalue_2) false false))

(fn FLoadNextPawn
  (bind _gameinstanacear (CallFunction|FGetGameInstance))
  (Variables|/Game/GameModes/Game_Instance_AR_Affordances.Game_Instance_AR_Affordances_C|SetCurrentPawn _gameinstanacear self)
  (Default|FMenuPawntoParticipantPawn _gameinstanacear))

(fn FGetNextInstructionsPage
  (params (ItemToFind :type E_Instructions_paths%20Enum :default "NewEnumerator0"))
  (bind _temprefarray (LocalVariables|GetTempRefArray))
  (bind _returnvalue (Utilities|Array|FindItem _temprefarray ItemToFind))
  (bind _returnvalue_2 (+ _returnvalue 1))
  (bind _output (Utilities|Array|Get(acopy) _temprefarray _returnvalue_2))
  (Utilities|Array|Clear _temprefarray)
  (bind _enumvalue (|ForEachE_Instructions_paths)
    (:LoopBody
      (Utilities|Array|Add _temprefarray _enumvalue))
    (:then
      (Math|Integer|CompareInt _returnvalue_2 (Utilities|Array|LastIndex _temprefarray)
        (:>
          (return _output true))
        (:==
          _)
        (:<
          _))
      (return _output false))))