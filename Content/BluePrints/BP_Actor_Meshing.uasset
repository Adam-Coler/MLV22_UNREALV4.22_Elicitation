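; Mixed-reality world meshing actor that scans the surroundings into an MRMesh with collision for queries and physics.
; BeginPlay connects the MeshTracker to the MRMesh, enables collision, and toggles scanning after a short delay.
; Toggle events flip the tracker's ScanWorld flag or swap the mesh between on and off materials to change its display.
; GetStatus builds a timestamped scan and display status string, printed when Verbose is set.
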(event Custom|Toggle_Scan
  (bind _meshtracker (Variables|Default|GetMeshTracker))
  ;[1 0.6657 0.4719] Toggle_Mesh_Scaning
  (if (Variables|/Script/MagicLeap.MeshTrackerComponent|GetScanWorld _meshtracker)
    (Variables|/Script/MagicLeap.MeshTrackerComponent|SetScanWorld _meshtracker false)
    (else
      (Variables|/Script/MagicLeap.MeshTrackerComponent|SetScanWorld _meshtracker true)))
  (CallFunction|GetStatus " Toggle_Scanning"))

(event Custom|Toggle_Mesh_Display
  (bind _mrmesh (Variables|Default|GetMRMesh))
  ;[0.9929 0.487 1] Toggle_Mesh_Display
  (if (Variables|View|GetIsMeshingDisplayed)
    (Rendering|Material|SetMaterial _mrmesh 0 (Variables|View|GetMeshing_Material_Off))
    (Variables|View|SetIsMeshingDisplayed false)
    (else
      (Rendering|Material|SetMaterial _mrmesh 0 (Variables|View|GetMeshing_Material_On))
      (Variables|View|SetIsMeshingDisplayed true)))
  (CallFunction|GetStatus " Toggle_Display"))

(event EventBeginPlay
  (bind _mrmesh (Variables|Default|GetMRMesh))
  ;[1 0.09928 0.189] Begin_Play
  (Utilities|FlowControl|Sequence
    (:then_0
      (Class|MeshTrackerComponent|ConnectMRMesh (Variables|Default|GetMeshTracker) _mrmesh))
    (:then_1
      (Collision|SetCollisionEnabled _mrmesh "QueryAndPhysics")
      (CallFunction|GetStatus " Begin_Play"))
    (:then_2
      (Utilities|FlowControl|Delay 1.0)
      (CallFunction|ToggleScan))))

(fn ConstructionScript)

(fn GetStatus
  (params (CalledFrom :type String))
  (bind _returnvalue (Utilities|Time|GetRealTimeSeconds))
  (bind _meshtracker (Variables|Default|GetMeshTracker))
  (bind _ismeshingdisplayed (Variables|View|GetIsMeshingDisplayed))
  (bind _returnvalue_2 (Utilities|String|ToString(Float) _returnvalue))
  (bind _returnvalue_3 (Utilities|String|ToString(Boolean) _ismeshingdisplayed))
  (bind _scanworld (Variables|/Script/MagicLeap.MeshTrackerComponent|GetScanWorld _meshtracker))
  (bind _returnvalue_4 (Utilities|String|ToString(Boolean) _scanworld))
  (bind _returnvalue_5 (Utilities|String|Append _returnvalue_2 " Uni: " "Meshing Actor " " Scanning:" _returnvalue_4 " Displaying: " _returnvalue_3 CalledFrom))
  (if (Variables|Default|GetVerbose)
    (Development|PrintString _returnvalue_5))
  (return _returnvalue_5))