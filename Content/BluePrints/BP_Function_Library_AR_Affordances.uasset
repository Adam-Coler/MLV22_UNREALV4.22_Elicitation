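; Blueprint function library for an AR affordances project, giving shared access to core game objects.
; Getters cast to the project's game mode and game instance, then read the shelf transform and gesture reader stored on the instance.
; A banner helper writes text to the game instance and fires its update dispatcher for widgets.
; Failed casts log through a print helper that prefixes real-time seconds and a tag.
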(fn FGetGameMode
  (bind _asgame_mode_ar_affordances (Utilities|Casting|CastToGame_Mode_AR_Affordances (Game|GetGameMode))
    (:then
      _)
    (:CastFailed
      (CallFunction|FPrint "GameMode Cast Failed")))
  (return _asgame_mode_ar_affordances))

(fn FPrint
  (params (PrintString :type String))
  (Development|PrintString 0 (Utilities|String|Append (Utilities|String|ToString(Float) (Utilities|Time|GetRealTimeSeconds)) " Uni: " PrintString)))

(fn FGetGameInstance
  (bind _asgame_instance_ar_affordances (Utilities|Casting|CastToGame_Instance_AR_Affordances (Game|GetGameInstance))
    (:then
      (return _asgame_instance_ar_affordances))
    (:CastFailed
      (CallFunction|FPrint "GameInstance Cast Failed"))))

(fn FGetShelfTransform
  (bind _gameinstanacear (CallFunction|FGetGameInstance))
  (return (Variables|/Game/GameModes/Game_Instance_AR_Affordances.Game_Instance_AR_Affordances_C|GetShelf_Transform _gameinstanacear)))

(fn FGetGestureReader
  (bind _gameinstanacear (CallFunction|FGetGameInstance))
  (bind _asbp_gesture_reader (Utilities|Casting|CastToBP_GestureReader (Variables|/Game/GameModes/Game_Instance_AR_Affordances.Game_Instance_AR_Affordances_C|GetGestureReader _gameinstanacear))
    (:then
      _)
    (:CastFailed
      (CallFunction|FPrint " Lib->GestureReaderBadCast")))
  (return _asbp_gesture_reader))

(fn FUpdateTextonWidgetViaEventDispatch
  (params (Text :type Text))
  (bind _gameinstanacear (CallFunction|FGetGameInstance))
  (Variables|/Game/GameModes/Game_Instance_AR_Affordances.Game_Instance_AR_Affordances_C|SetBannerText _gameinstanacear Text)
  (Default|CallBannerUpdate _gameinstanacear))